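; BP_Piece is a collectible coin pickup that loops its animation from BeginPlay.
; When BP_ThirdPersonCharacter overlaps its Sphere, it increments that character's Coins, plays a coin sound at its location and activates a Niagara effect.
; It then destroys the Piece and Sphere components at once, delaying actor destruction by two seconds after the effect starts.
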(event `self.ReceiveBeginPlay`
  (`SkeletalMeshComponent.PlayAnimation` (`self.piece`) "/Game/Assets/Object/Piece/piece_Anim.piece_Anim" true))

(event `self.Sphere.OnComponentBeginOverlap`
  (params (OverlappedComponent :type "PrimitiveComponent Object Reference") (OtherActor :type "Actor Object Reference") (OtherComp :type "PrimitiveComponent Object Reference") (OtherBodyIndex :type Integer) (bFromSweep :type Boolean) (SweepResult :type "HitResult Structure (by ref)"))
  (bind _asbp_third_person_character (cast `/Game/ThirdPerson/Blueprints/BP_ThirdPersonCharacter` OtherActor))
  (`/Engine/EditorBlueprintResources/StandardMacros.IncrementInt` (`/Game/ThirdPerson/Blueprints/BP_ThirdPersonCharacter.Coins` _asbp_third_person_character)
    (:`  `
      (`GameplayStatics.PlaySoundAtLocation` "/Game/SFX/Piece/drop-coin-384921.drop-coin-384921" (`self.K2_GetActorLocation`) (struct) 1.0 1.0 0.0 null null null null)
      (`ActorComponent.Activate` (`self.Niagara`) true)
      (`ActorComponent.K2_DestroyComponent` (`self.piece`))
      (`ActorComponent.K2_DestroyComponent` (`self.Sphere`))
      (`KismetSystemLibrary.Delay` 2.0)
      (`self.K2_DestroyActor`))))

(fn `UserConstructionScript`)