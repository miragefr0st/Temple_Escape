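; BP_FlyingZone is a box volume actor that supplies random 3D points inside its bounds, apparently as targets for flying movement.
; On BeginPlay it caches the collision component's box extent and the actor's location.
; GetRandomPoint picks each axis independently within location plus or minus extent, so results are axis-aligned and centred on the actor's cached position.
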(event `self.ReceiveBeginPlay`
  (set `self.Box Extent` (`.BoxExtent` (`KismetSystemLibrary.GetComponentBounds` (`self.CollisionComponent`))))
  (set `self.ActorLocation` (`self.K2_GetActorLocation`)))

(fn `GetRandomPoint`
  (returns (RandomPoint :type "Vector Structure"))
  (bind (_actorlocation_x _actorlocation_y _actorlocation_z) (`KismetMathLibrary.BreakVector` (`self.ActorLocation`)))
  (bind (_box_extent_x _box_extent_y _box_extent_z) (`KismetMathLibrary.BreakVector` (`self.Box Extent`)))
  (bind _actorlocation_x_2 (`KismetMathLibrary.BreakVector` (`self.ActorLocation`)))
  (bind _box_extent_x_2 (`KismetMathLibrary.BreakVector` (`self.Box Extent`)))
  (bind (_actorlocation_x_3 _actorlocation_y_2) (`KismetMathLibrary.BreakVector` (`self.ActorLocation`)))
  (bind (_box_extent_x_3 _box_extent_y_2) (`KismetMathLibrary.BreakVector` (`self.Box Extent`)))
  (return (`KismetMathLibrary.MakeVector` (`KismetMathLibrary.RandomFloatInRange` (- _actorlocation_x_2 _box_extent_x_2) (+ _actorlocation_x_2 _box_extent_x_2)) (`KismetMathLibrary.RandomFloatInRange` (- _actorlocation_y_2 _box_extent_y_2) (+ _actorlocation_y_2 _box_extent_y_2)) (`KismetMathLibrary.RandomFloatInRange` (- _actorlocation_z _box_extent_z) (+ _actorlocation_z _box_extent_z)))))

(fn `UserConstructionScript`)