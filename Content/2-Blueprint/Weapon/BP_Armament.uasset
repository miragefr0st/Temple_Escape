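; BP_Armament is a proximity weapon that damages and knocks back BP_ThirdPersonCharacter when it enters the detection sphere.
; BeginPlay applies the configured mesh and range after a short delay.
; PlayerInRange plays a sound, hits and launches the player, then starts a reload, or schedules a delayed retry if already reloading.
; Tick counts down FireRate with DoOnce gates and re-attacks while IsInRange, which end overlap also sets true.
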(event `self.ReceiveBeginPlay`
  (`KismetSystemLibrary.Delay` 0.2)
  (`StaticMeshComponent.SetStaticMesh` (`self.StaticMesh`) (`self.Mesh`))
  (`SphereComponent.SetSphereRadius` (`self.DetectionRange`) (`self.Range`) true)
  (set `self.SaveRate` (`self.FireRate`)))

(event `self.DetectionRange.OnComponentBeginOverlap`
  (params (OverlappedComponent :type "PrimitiveComponent Object Reference") (OtherActor :type "Actor Object Reference") (OtherComp :type "PrimitiveComponent Object Reference") (OtherBodyIndex :type Integer) (bFromSweep :type Boolean) (SweepResult :type "HitResult Structure (by ref)"))
  (bind _asbp_third_person_character (cast `/Game/ThirdPerson/Blueprints/BP_ThirdPersonCharacter` OtherActor))
  (bind _output_get (set `self.As BP Third Person Character` _asbp_third_person_character))
  (set `self.IsInRange` true)
  (`self.PlayerInRange` _output_get))

(event `self.DetectionRange.OnComponentEndOverlap`
  (params (OverlappedComponent :type "PrimitiveComponent Object Reference") (OtherActor :type "Actor Object Reference") (OtherComp :type "PrimitiveComponent Object Reference") (OtherBodyIndex :type Integer))
  (cast `/Game/ThirdPerson/Blueprints/BP_ThirdPersonCharacter` OtherActor)
  (set `self.IsInRange` true))

(event `self.ReceiveTick`
  (params (DeltaSeconds :type "Float (single-precision)"))
  (bind _saverate (`self.SaveRate`))
  (if (> _saverate 0.0)
    (bind _output_get (set `self.SaveRate` (- _saverate DeltaSeconds)))
    (if (<= _output_get 0.0)
      (`|ExecutionSequence`
        (:`then_0`
          (`/Engine/EditorBlueprintResources/StandardMacros.DoOnce` false :!label _label
            (:`Completed`
              (set `self.IsReloading` false))))
        (:`then_1`
          (`/Engine/EditorBlueprintResources/StandardMacros.DoOnce` false :!label _label_2
            (:`Completed`
              (if (`self.IsInRange`)
                (`self.PlayerInRange` (`self.As BP Third Person Character`))))))))))

(event `ResetOnce`
  (`|ExecutionSequence`
    (:`then_0`
      (goto _label :!via `Reset`))
    (:`then_1`
      (goto _label_2 :!via `Reset`))))

(event `HitANewTime`
  (bind _as_bp_third_person_character (`self.As BP Third Person Character`))
  (`/Engine/EditorBlueprintResources/StandardMacros.IsValid` _as_bp_third_person_character
    (:`Is Valid`
      (`KismetSystemLibrary.Delay` (`self.SaveRate`))
      (`self.PlayerInRange` _as_bp_third_person_character))))

(fn `ApplyDamage`
  (`/Game/ThirdPerson/Blueprints/BP_ThirdPersonCharacter.HitPlayer` (`self.As BP Third Person Character`)))

(fn `KnockBack`
  (bind _as_bp_third_person_character (`self.As BP Third Person Character`))
  (`Character.LaunchCharacter` _as_bp_third_person_character (* (`KismetMathLibrary.Normal` (- (`self.K2_GetActorLocation` _as_bp_third_person_character) (`self.K2_GetActorLocation` self))) (`self.KnockBackRange`)) false false))

(fn `PlayerInRange`
  (params (Player :type "/Game/ThirdPerson/Blueprints/BP_ThirdPersonCharacter Object Reference"))
  (if (`self.IsReloading`)
    (`self.HitANewTime`)
    (else
      (`GameplayStatics.PlaySoundAtLocation` (`self.Sound`) (`self.K2_GetActorLocation`) (struct) 500.0 1.0 0.0 null null null null)
      (`/Game/ThirdPerson/Blueprints/BP_ThirdPersonCharacter.HitPlayer` Player)
      (`self.KnockBack`)
      (set `self.IsReloading` true)
      (set `self.SaveRate` (`self.FireRate`))
      (`self.ResetOnce`))))

(fn `UserConstructionScript`)