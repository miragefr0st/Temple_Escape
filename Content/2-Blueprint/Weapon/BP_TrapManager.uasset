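; BP_TrapManager is a trap manager that spawns, tracks and deletes trap weapons.
; Both add functions read a TrapDataTable row, spawn its weapon class, store it in TrapArray and copy stats onto it as BP_Armament.
; AddTrap spawns at the manager's transform, while AddTrapRandomPoint uses a BP_FlyingZone navmesh point and leaves FireRate unset.
; DeleteTrap destroys the trap at index TrapToDelete and removes it from the array.
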(fn `AddTrap`
  (bind _returnvalue (`|GetDataTableRow` (`self.TrapDataTable`) (`.RowName` (break `DataTableRowHandle` (`self.Traps`))))
    (:`then`
      (bind (_weaponclass _weaponname _firerate _range _knowkback _mesh _sound) (break `/Game/2-Blueprint/Weapon/WeaponStruct` _returnvalue))
      (bind _returnvalue_2 (`|SpawnActorFromClass` _weaponclass (`self.GetTransform`) "AdjustIfPossibleButAlwaysSpawn" "MultiplyWithRoot" null _weaponname _range null))
      (`KismetArrayLibrary.Array_Add` (`self.TrapArray`) _returnvalue_2)
      (bind _asbp_armament (cast `/Game/2-Blueprint/Weapon/BP_Armament` _returnvalue_2))
      (set `/Game/2-Blueprint/Weapon/BP_Armament.FireRate` _firerate _asbp_armament)
      (set `/Game/2-Blueprint/Weapon/BP_Armament.Mesh` _mesh _asbp_armament)
      (set `/Game/2-Blueprint/Weapon/BP_Armament.KnockBackRange` _knowkback _asbp_armament)
      (set `/Game/2-Blueprint/Weapon/BP_Armament.Sound` _sound _asbp_armament))))

(fn `AddTrapRandomPoint`
  (bind _returnvalue (`|GetDataTableRow` (`self.TrapDataTable`) (`.RowName` (break `DataTableRowHandle` (`self.Traps`))))
    (:`then`
      (bind _returnvalue_2 (`GameplayStatics.GetActorOfClass` "/Game/2-Blueprint/BP_FlyingZone.BP_FlyingZone_C"))
      (bind _randompoint (`/Game/2-Blueprint/BP_FlyingZone.GetPointInNavMesh` _returnvalue_2))
      (bind (_weaponclass _weaponname _firerate _range _knowkback _mesh _sound) (break `/Game/2-Blueprint/Weapon/WeaponStruct` _returnvalue))
      (bind _returnvalue_3 (`|SpawnActorFromClass` _weaponclass (`KismetMathLibrary.Conv_VectorToTransform` _randompoint) "AdjustIfPossibleButAlwaysSpawn" "MultiplyWithRoot" null _weaponname _range null))
      (`KismetArrayLibrary.Array_Add` (`self.TrapArray`) _returnvalue_3)
      (bind _asbp_armament (cast `/Game/2-Blueprint/Weapon/BP_Armament` _returnvalue_3))
      (set `/Game/2-Blueprint/Weapon/BP_Armament.Mesh` _mesh _asbp_armament)
      (set `/Game/2-Blueprint/Weapon/BP_Armament.KnockBackRange` _knowkback _asbp_armament)
      (set `/Game/2-Blueprint/Weapon/BP_Armament.Sound` _sound _asbp_armament))))

(fn `DeleteTrap`
  (bind _output (`|GetArrayItem` (`self.TrapArray`) (`self.TrapToDelete`)))
  (`self.K2_DestroyActor` _output)
  (`KismetArrayLibrary.Array_RemoveItem` (`self.TrapArray`) _output))

(fn `UserConstructionScript`)