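; BP_Armament is a weapon or hazard actor that repeatedly damages and knocks back the third-person player character while it stays inside a detection sphere.
; BeginPlay waits briefly, then applies the configured mesh and detection radius.
; Overlap calls HitPlayer and launches the character away from the actor, then repeats both on a looping FireRate timer.
; Leaving the sphere clears that timer.
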(event `self.ReceiveBeginPlay`
  (`KismetSystemLibrary.Delay` 0.2)
  (`StaticMeshComponent.SetStaticMesh` (`self.StaticMesh`) (`self.Mesh`))
  (`SphereComponent.SetSphereRadius` (`self.DetectionRange`) (`self.Range`) true))

(event `self.DetectionRange.OnComponentBeginOverlap`
  (params (OverlappedComponent :type "PrimitiveComponent Object Reference") (OtherActor :type "Actor Object Reference") (OtherComp :type "PrimitiveComponent Object Reference") (OtherBodyIndex :type Integer) (bFromSweep :type Boolean) (SweepResult :type "HitResult Structure (by ref)"))
  (bind _asbp_third_person_character (cast `/Game/ThirdPerson/Blueprints/BP_ThirdPersonCharacter` OtherActor))
  (bind _output_get (set `self.As BP Third Person Character` _asbp_third_person_character))
  (`self.ApplyDamage` _output_get)
  (`self.KnockBack`)
  (bind _returnvalue (`KismetSystemLibrary.K2_SetTimerDelegate` (delegate `EventTimer`) (`self.FireRate`) true))
  (set `self.DamageTimerHandle` _returnvalue))

(event `EventTimer`
  (`self.ApplyDamage` (`self.As BP Third Person Character`))
  (`self.KnockBack`))

(event `self.DetectionRange.OnComponentEndOverlap`
  (params (OverlappedComponent :type "PrimitiveComponent Object Reference") (OtherActor :type "Actor Object Reference") (OtherComp :type "PrimitiveComponent Object Reference") (OtherBodyIndex :type Integer))
  (cast `/Game/ThirdPerson/Blueprints/BP_ThirdPersonCharacter` OtherActor)
  (`KismetSystemLibrary.K2_ClearAndInvalidateTimerHandle` (`self.DamageTimerHandle`)))

(fn `ApplyDamage`
  (params (Target :type "/Game/ThirdPerson/Blueprints/BP_ThirdPersonCharacter Object Reference"))
  (`/Game/ThirdPerson/Blueprints/BP_ThirdPersonCharacter.HitPlayer` Target))

(fn `KnockBack`
  (bind _as_bp_third_person_character (`self.As BP Third Person Character`))
  (`Character.LaunchCharacter` _as_bp_third_person_character (* (`KismetMathLibrary.Normal` (- (`self.K2_GetActorLocation` _as_bp_third_person_character) (`self.K2_GetActorLocation` self))) (`self.KnockBackRange`)) false false))

(fn `UserConstructionScript`)