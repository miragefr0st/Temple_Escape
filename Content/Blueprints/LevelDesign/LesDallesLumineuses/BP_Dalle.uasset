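; BP_Dalle is a glowing floor tile from the LesDallesLumineuses level-design set, meant to light up temporarily.
; On BeginPlay it gives the Dalle component a dynamic material instance and zeroes its Color parameter.
; LightUp, which nothing here calls, writes emissive scalar parameters, then waits two seconds.
; The closing reset targets a parameter named None, so it does not undo the emissive writes.
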(event `self.ReceiveBeginPlay`
  (bind _dalle (`self.dalle`))
  (bind _returnvalue (`PrimitiveComponent.CreateDynamicMaterialInstance` _dalle 0 (`PrimitiveComponent.GetMaterial` _dalle 0) "None"))
  (set `self.Material` _returnvalue)
  (`PrimitiveComponent.SetMaterial` (`self.dalle`) 0 _returnvalue)
  (`MaterialInstanceDynamic.SetScalarParameterValue` (`self.Material`) "Color" 0.0))

(event `LightUp`
  (`MaterialInstanceDynamic.SetScalarParameterValue` (`self.Material`) (`self.EmissiveIntensity`) (`self.EmissiveColor`))
  (`MaterialInstanceDynamic.SetScalarParameterValue` (`self.Material`) "EmissiveColor" 0.0)
  (`KismetSystemLibrary.Delay` 2.0)
  (`MaterialInstanceDynamic.SetScalarParameterValue` (`self.Material`) "None" 0.0))

(fn `UserConstructionScript`)