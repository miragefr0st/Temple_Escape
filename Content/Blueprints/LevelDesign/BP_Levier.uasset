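; BP_Levier is a toggleable level-design lever that switches a linked object on and off.
; Its box overlap registers the lever as the third-person character's CurrentInteractable and clears it on exit.
; Each Interact plays a sound, flips the On state, calls Activate or Deactivate on Link, and plays or reverses a timeline meant to rotate the lever bar.
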(event `/Game/ThirdPerson/Blueprints/BPI_CharacterInterface.Interact`
  (bind _link (`self.Link`))
  (bind _t_movelevier (`self.T_MoveLevier`))
  ; Event Interact
  (`GameplayStatics.PlaySound2D` "/Game/SFX/LevierCue.LevierCue" 1.0 1.0 0.0 null null)
  (bind _output_get (set `self.On` (not (`self.On`))))
  (if _output_get
    (`TimelineComponent.Play` _t_movelevier)
    (`/Game/Blueprints/LevelDesign/BP_Activable_Interface.Activate` _link)
    (else
      (`TimelineComponent.Reverse` _t_movelevier)
      (`/Game/Blueprints/LevelDesign/BP_Activable_Interface.Deactivate` _link))))

(event `self.Box.OnComponentBeginOverlap`
  (params (OverlappedComponent :type "PrimitiveComponent Object Reference") (OtherActor :type "Actor Object Reference") (OtherComp :type "PrimitiveComponent Object Reference") (OtherBodyIndex :type Integer) (bFromSweep :type Boolean) (SweepResult :type "HitResult Structure (by ref)"))
  (bind _asbp_third_person_character (cast `/Game/ThirdPerson/Blueprints/BP_ThirdPersonCharacter` OtherActor))
  (set `/Game/ThirdPerson/Blueprints/BP_ThirdPersonCharacter.CurrentInteractable` self _asbp_third_person_character))

(event `self.Box.OnComponentEndOverlap`
  (params (OverlappedComponent :type "PrimitiveComponent Object Reference") (OtherActor :type "Actor Object Reference") (OtherComp :type "PrimitiveComponent Object Reference") (OtherBodyIndex :type Integer))
  (bind _asbp_third_person_character (cast `/Game/ThirdPerson/Blueprints/BP_ThirdPersonCharacter` OtherActor))
  (set `/Game/ThirdPerson/Blueprints/BP_ThirdPersonCharacter.CurrentInteractable` null _asbp_third_person_character))

(fn `UserConstructionScript`)