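; BP_LightRay is a light beam actor for what appears to be a mirror-and-receptacle light puzzle.
; SpawnSpline line-traces forward, records an inactive mirror or a receptacle as connected, and stretches the spline mesh to that target's arrow or the trace end point.
; A timeline fades the beam's dynamic material alpha, activating the connected target when charging finishes.
; A disconnect event deactivates and clears connected targets.
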(event `self.ReceiveBeginPlay`
  (bind _returnvalue (`PrimitiveComponent.CreateDynamicMaterialInstance` (`self.SplineMesh`) 0 "/Game/Materials/RayonsLumineux/M_LightRay.M_LightRay" "None"))
  (set `self.RayMaterial` _returnvalue))

(event `Event ChargeLight`
  (params (Inverse :type Boolean))
  (bind _connectedmirror (`self.ConnectedMirror`))
  (bind _connectedreceptacle (`self.ConnectedReceptacle`))
  (if Inverse
    (bind (_direction _alpha) (`Timeline|Timeline` :!via `Reverse` :!label _label)
      (:`Update`
        (`MaterialInstanceDynamic.SetScalarParameterValue` (`self.RayMaterial`) "P_Alpha" _alpha))
      (:`Finished`
        (if (not Inverse)
          (`/Engine/EditorBlueprintResources/StandardMacros.IsValid` _connectedmirror
            (:`Is Valid`
              (`/Game/Blueprints/LevelDesign/RayonsLumineux/BP_Mirroir.Activate` _connectedmirror))
            (:`Is Not Valid`
              _))
          (`/Engine/EditorBlueprintResources/StandardMacros.IsValid` _connectedreceptacle
            (:`Is Valid`
              (`/Game/Blueprints/LevelDesign/RayonsLumineux/BP_ReceptacleLumiere.Event_Activate` _connectedreceptacle))))))
    (else
      (goto _label))))

(event `Event_DisconnectMirror`
  (bind _connectedreceptacle (`self.ConnectedReceptacle`))
  (bind _connectedmirror (`self.ConnectedMirror`))
  (`/Engine/EditorBlueprintResources/StandardMacros.IsValid` _connectedmirror
    (:`Is Valid`
      (`/Game/Blueprints/LevelDesign/RayonsLumineux/BP_Mirroir.Deactivate` _connectedmirror)
      (set `self.ConnectedMirror` null))
    (:`Is Not Valid`
      _))
  (`/Engine/EditorBlueprintResources/StandardMacros.IsValid` _connectedreceptacle
    (:`Is Valid`
      (`/Game/Blueprints/LevelDesign/RayonsLumineux/BP_ReceptacleLumiere.Event_Deactivate` _connectedreceptacle)
      (set `self.ConnectedReceptacle` null))))

(fn `SpawnSpline`
  (params (StartPos :type "Vector Structure") (Forward :type "Vector Structure") (StartActor :type "Actor Object Reference"))
  (locals (Length :type "Float (double-precision)" :default 2000.0) (RayEnd :type "Vector Structure") (RayMaxLength :type "Vector Structure") (Start :type "Vector Structure"))
  (bind _start (`local.Start`))
  (bind _output_get (set `local.Start` StartPos))
  (bind _outhit (`KismetSystemLibrary.LineTraceSingle` _output_get (+ StartPos (* Forward (`local.Length`))) "TraceTypeQuery2" false (`|MakeArray` StartActor self :!type "Actor Object Reference") "ForDuration" true (struct :`R` 1.0 :`B` 0.555737 :`A` 1.0) (struct :`R` 1.0 :`G` 0.907297 :`A` 1.0)))
  (bind (_bblockinghit _binitialoverlap _time _distance _location _impactpoint _normal _impactnormal _physmat _hitactor _hitcomponent _hitbonename _bonename _hititem _elementindex _faceindex _tracestart _traceend) (`GameplayStatics.BreakHitResult` _outhit))
  (if _bblockinghit
    (bind _asbp_mirroir (cast `/Game/Blueprints/LevelDesign/RayonsLumineux/BP_Mirroir` _hitactor)
      (:`then`
        (if (not (`/Game/Blueprints/LevelDesign/RayonsLumineux/BP_Mirroir.activated` _asbp_mirroir))
          (set `self.ConnectedMirror` _asbp_mirroir)
          (`self.UpdateSplineMesh` _start (`SceneComponent.K2_GetComponentLocation` (`/Game/Blueprints/LevelDesign/RayonsLumineux/BP_Mirroir.Arrow` _asbp_mirroir)))))
      (:`CastFailed`
        (bind _asbp_receptacle_lumiere (cast `/Game/Blueprints/LevelDesign/RayonsLumineux/BP_ReceptacleLumiere` _hitactor)
          (:`then`
            (set `self.ConnectedReceptacle` _asbp_receptacle_lumiere)
            (`self.UpdateSplineMesh` _start (`SceneComponent.K2_GetComponentLocation` (`/Game/Blueprints/LevelDesign/RayonsLumineux/BP_ReceptacleLumiere.Arrow` _asbp_receptacle_lumiere))))
          (:`CastFailed`
            (`self.UpdateSplineMesh` _start _impactpoint)))))
    (else
      (`self.UpdateSplineMesh` _start _traceend))))

(fn `UpdateSplineMesh`
  (params (Start :type "Vector Structure") (End :type "Vector Structure"))
  (`SplineMeshComponent.SetEndPosition` (`self.SplineMesh`) (`KismetMathLibrary.InverseTransformLocation` (`self.GetTransform`) End) true)
  (`self.Event ChargeLight` false))

(fn `UserConstructionScript`)