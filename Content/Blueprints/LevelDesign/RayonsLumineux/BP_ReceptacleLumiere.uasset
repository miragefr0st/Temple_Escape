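; Light receptacle for the light-ray level design elements, acting as a switch that relays its on/off state to a target.
; Its Activate and Deactivate events fire the TurnOnOff dispatcher, then forward the same call to Target if it implements the interface.
; It binds to its own dispatcher on BeginPlay, only to print the light state for debugging.
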(event `self.ReceiveBeginPlay`
  (add `self.TurnOnOff` (delegate `TurnOnOff_Event`)))

(event `TurnOnOff_Event` :!signature `self.TurnOnOff`
  (params (On :type Boolean))
  (if On
    (`KismetSystemLibrary.PrintString` "Light On!")
    (else
      (`KismetSystemLibrary.PrintString` "Light Off!"))))

(event `Event_Activate`
  (bind _target (`self.Target`))
  (`self.TurnOnOff` true)
  (if (`KismetSystemLibrary.IsValidInterface` _target)
    (`/Game/Blueprints/LevelDesign/BP_Activable_Interface.Activate` _target)))

(event `Event_Deactivate`
  (bind _target (`self.Target`))
  (`self.TurnOnOff` false)
  (if (`KismetSystemLibrary.IsValidInterface` _target)
    (`/Game/Blueprints/LevelDesign/BP_Activable_Interface.Deactivate` _target)))

(fn `UserConstructionScript`)