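; BP_LighthManager is a light manager in the light-ray level design folder that shows or hides a set of light actors.
; When Activation is off, BeginPlay binds its Light event to a Trigger's on/off dispatcher.
; Light, Activate and Deactivate loop over the Lights array, setting root component visibility with propagation to children.
; Light also maintains a Working flag, while leftover delay-scaling logic is disconnected.
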(event `self.ReceiveBeginPlay`
  (if (not (`self.Activation`))
    (add `/Game/Blueprints/LevelDesign/RayonsLumineux/BP_ReceptacleLumiere.TurnOnOff` (`self.Trigger`) (delegate `Light`))))

(event `Light`
  (params (On :type Boolean))
  (if On
    (set `self.Working` true)
    (for _array_element (`self.Lights`)
      (`SceneComponent.SetVisibility` (`Actor.RootComponent` _array_element) true true)
      (`KismetSystemLibrary.Delay` 120.0))
    (set `self.Working` false :!label _label)
    (else
      (for _array_element_2 (`self.Lights`)
        (`SceneComponent.SetVisibility` (`Actor.RootComponent` _array_element_2) false true)
        (goto _label)))))

(event `/Game/Blueprints/LevelDesign/BP_Activable_Interface.Activate`
  (for _array_element (`self.Lights`)
    (`SceneComponent.SetVisibility` (`Actor.RootComponent` _array_element) true true)))

(event `/Game/Blueprints/LevelDesign/BP_Activable_Interface.Deactivate`
  (for _array_element (`self.Lights`)
    (`SceneComponent.SetVisibility` (`Actor.RootComponent` _array_element) false true)))

(fn `UserConstructionScript`)