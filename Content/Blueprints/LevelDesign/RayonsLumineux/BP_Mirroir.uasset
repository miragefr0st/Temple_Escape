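; Rotatable mirror for a light-ray puzzle that emits its own ray while activated.
; Interact cycles the mirror rotator through an array of preset rotations, wrapping at the end, and re-casts the ray if active.
; A child-actor BP_LightRay, cached at BeginPlay, spawns its spline from the Arrow's position and forward vector on Activate.
; Deactivate calls the ray's charge-light and disconnect-mirror events and clears the active flag.
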(event `self.ReceiveBeginPlay`
  (`SceneComponent.K2_SetRelativeRotation` (`self.MirrorRotator`) (`|GetArrayItem` (`self.Rotations`) (`self.Index`)) false false)
  (bind _asbp_light_ray (cast `/Game/Blueprints/LevelDesign/RayonsLumineux/BP_LightRay` (`ChildActorComponent.ChildActor` (`self.BP_LightRay`))))
  (set `self.LightRay` _asbp_light_ray))

(event `PlayerInteraction_Interface.Interact`
  (bind _arrow (`self.Arrow`))
  (bind _lightray (`self.LightRay`))
  (if (== (`self.Index`) (- (`KismetArrayLibrary.Array_Length` (`self.Rotations`)) 1))
    (set `self.Index` 0)
    (else
      (set `self.Index` (+ (`self.Index`) 1))))
  (`SceneComponent.K2_SetRelativeRotation` (`self.MirrorRotator`) (`|GetArrayItem` (`self.Rotations`) (`self.Index`)) false false)
  (if (`self.activated`)
    (`/Game/Blueprints/LevelDesign/RayonsLumineux/BP_LightRay.Event_DisconnectMirror` _lightray)
    (`/Game/Blueprints/LevelDesign/RayonsLumineux/BP_LightRay.SpawnSpline` _lightray (`SceneComponent.K2_GetComponentLocation` _arrow) (`SceneComponent.GetForwardVector` _arrow) self)))

(fn `Activate`
  (bind _arrow (`self.Arrow`))
  (`/Game/Blueprints/LevelDesign/RayonsLumineux/BP_LightRay.SpawnSpline` (`self.LightRay`) (`SceneComponent.K2_GetComponentLocation` _arrow) (`SceneComponent.GetForwardVector` _arrow) self)
  (set `self.activated` true))

(fn `Deactivate`
  (bind _lightray (`self.LightRay`))
  (`/Game/Blueprints/LevelDesign/RayonsLumineux/BP_LightRay.Event ChargeLight` _lightray true)
  (set `self.activated` false)
  (`/Game/Blueprints/LevelDesign/RayonsLumineux/BP_LightRay.Event_DisconnectMirror` _lightray))

(fn `UserConstructionScript`)