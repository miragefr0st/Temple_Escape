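; BP_UpDowner is a level trap actor that moves continuously up and down from its placed position.
; BeginPlay records the start location, then enables motion after a configurable delay so the movement can begin later.
; Tick accumulates time and lerps between the start and a point Height above it, using the absolute sine in degrees of time times Speed, with sweep enabled.
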(event `self.ReceiveBeginPlay`
  (set `self.StartPos` (`self.K2_GetActorLocation` (`self.Actor`)))
  (`KismetSystemLibrary.Delay` (`self.Delay`))
  (set `self.Start` true))

(event `self.ReceiveTick`
  (params (DeltaSeconds :type "Float (single-precision)"))
  (bind (_startpos_x _startpos_y _startpos_z) (`KismetMathLibrary.BreakVector` (`self.StartPos`)))
  (if (`self.Start`)
    (set `self.time` (+ DeltaSeconds (`self.time`)))
    (`self.K2_SetActorLocation` (`self.Actor`) (`KismetMathLibrary.VLerp` (`self.StartPos`) (`KismetMathLibrary.MakeVector` _startpos_x _startpos_y (+ _startpos_z (`self.Height`))) (`KismetMathLibrary.Abs` (`KismetMathLibrary.DegSin` (* (`self.time`) (`self.Speed`))))) true false)))

(fn `UserConstructionScript`)