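; A trap platform that slides aside along world Y when an actor overlaps it, then returns.
; An overlap starts the Retract timeline, moving the actor by its Y size left or right per GoRight; after three seconds RetractReverse moves it back.
; A Moving flag blocks retriggering mid-cycle, and Speed scales the lerp alpha rather than timeline play rate.
; The construction script sizes the cube and trigger box from variables.
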(event `self.ReceiveBeginPlay`
  (`SceneComponent.SetRelativeScale3D` (`self.Cube`) (`self.Size`))
  (set `self.StartPos` (`self.K2_GetActorLocation`)))

(event `self.ReceiveActorBeginOverlap`
  (params (OtherActor :type "Actor Object Reference"))
  (bind (_startpos_x _startpos_y _startpos_z) (`KismetMathLibrary.BreakVector` (`self.StartPos`)))
  (bind (_size_x _size_y) (`KismetMathLibrary.BreakVector` (`self.Size`)))
  (bind (_size_x_2 _size_y_2) (`KismetMathLibrary.BreakVector` (`self.Size`)))
  (bind (_startpos_x_2 _startpos_y_2 _startpos_z_2) (`KismetMathLibrary.BreakVector` (`self.StartPos`)))
  (if (not (`self.Moving`))
    (set `self.Moving` true)
    (bind (_direction _alpha) (`Timeline|Retract` :!via `PlayFromStart`)
      (:`Update`
        (if (`self.GoRight`)
          (bind _returnvalue (* (`self.Speed`) _alpha))
          (`self.K2_SetActorLocation` (`KismetMathLibrary.VLerp` (`self.StartPos`) (`KismetMathLibrary.MakeVector` _startpos_x (- _startpos_y (* _size_y 100.0)) _startpos_z) _returnvalue))
          (else
            (`self.K2_SetActorLocation` (`KismetMathLibrary.VLerp` (`self.StartPos`) (`KismetMathLibrary.MakeVector` _startpos_x_2 (+ _startpos_y_2 (* _size_y_2 100.0)) _startpos_z_2) _returnvalue)))))
      (:`Finished`
        (set `self.CurrentPos` (`self.K2_GetActorLocation`))
        (`KismetSystemLibrary.Delay` 3.0)
        (bind (_direction_2 _alpha_2) (`Timeline|RetractReverse` :!via `PlayFromStart`)
          (:`Update`
            (`self.K2_SetActorLocation` (`KismetMathLibrary.VLerp` (`self.CurrentPos`) (`self.StartPos`) (* (`self.Speed`) _alpha_2))))
          (:`Finished`
            (set `self.Moving` false)))))))

(fn `UserConstructionScript`
  (`SceneComponent.SetRelativeScale3D` (`self.Cube`) (`self.Size`))
  (`SceneComponent.K2_SetRelativeLocation` (`self.Box`) (`KismetMathLibrary.MakeVector` 0.0 0.0 (`self.ColliderHeight`)) false false)
  (`BoxComponent.SetBoxExtent` (`self.Box`) (`self.ColliderSize`) true))