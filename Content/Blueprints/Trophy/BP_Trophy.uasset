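; Collectible trophy actor that spins in place and is picked up when the player character touches it.
; It plays an attenuated shine sound on BeginPlay and rotates around its yaw axis each Tick.
; On Cube overlap, it passes the game mode's trophy count to the character's WidgetInterface, then increments that count.
; It then plays a pickup sound and destroys itself after a brief delay.
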(event `self.ReceiveBeginPlay`
  (`GameplayStatics.PlaySoundAtLocation` "/Game/SFX/Trophy/SC_TrophyShine.SC_TrophyShine" (`self.K2_GetActorLocation`) (struct) 1.0 1.0 0.0 "/Game/SFX/Trophy/SA_Trophy.SA_Trophy" null null null))

(event `self.Cube.OnComponentBeginOverlap`
  (params (OverlappedComponent :type "PrimitiveComponent Object Reference") (OtherActor :type "Actor Object Reference") (OtherComp :type "PrimitiveComponent Object Reference") (OtherBodyIndex :type Integer) (bFromSweep :type Boolean) (SweepResult :type "HitResult Structure (by ref)"))
  (bind _asbp_third_person_character (cast `/Game/ThirdPerson/Blueprints/BP_ThirdPersonCharacter` OtherActor))
  (bind _asbp_third_person_game_mode (cast `/Game/ThirdPerson/Blueprints/BP_ThirdPersonGameMode` (`GameplayStatics.GetGameMode`)))
  (bind _trophy (`/Game/ThirdPerson/Blueprints/BP_ThirdPersonGameMode.Trophy` _asbp_third_person_game_mode))
  (`/Game/UI/WidgetBlueprint/WBP_UserInterface.AddTrophy` (`/Game/ThirdPerson/Blueprints/BP_ThirdPersonCharacter.WidgetInterface` _asbp_third_person_character) _trophy)
  (`/Engine/EditorBlueprintResources/StandardMacros.IncrementInt` _trophy
    (:`  `
      (`GameplayStatics.PlaySoundAtLocation` "/Game/SFX/Trophy/freesound_gamestudio-get-item-394523.freesound_gamestudio-get-item-394523" (`self.K2_GetActorLocation`) (struct) 1.0 1.0 0.0 "/Game/SFX/Trophy/SA_Trophy.SA_Trophy" null null null)
      (`KismetSystemLibrary.Delay` 0.1)
      (`self.K2_DestroyActor`))))

(event `self.ReceiveTick`
  (params (DeltaSeconds :type "Float (single-precision)"))
  (`self.K2_AddActorLocalRotation` (`KismetMathLibrary.MakeRotator` 0.0 0.0 (* DeltaSeconds (`self.RotationSpeed`)))))

(fn `UserConstructionScript`)