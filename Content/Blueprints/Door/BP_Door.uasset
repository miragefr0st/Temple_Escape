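; BP_Door is an automatic door that opens when the third-person character enters its Box trigger and closes when they leave.
; The overlap events play and reverse the door timeline through its component reference.
; The timeline's update logic lerps the Cylinder's relative yaw toward OpenAngle and its relative location toward OpenPos, combining swing and slide.
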(event `self.Box.OnComponentBeginOverlap`
  (params (OverlappedComponent :type "PrimitiveComponent Object Reference") (OtherActor :type "Actor Object Reference") (OtherComp :type "PrimitiveComponent Object Reference") (OtherBodyIndex :type Integer) (bFromSweep :type Boolean) (SweepResult :type "HitResult Structure (by ref)"))
  ; Open The Door if The Player Overlap the Box
  (cast `/Game/ThirdPerson/Blueprints/BP_ThirdPersonCharacter` OtherActor)
  (`TimelineComponent.Play` (`self.TL_Door`)))

(event `self.Box.OnComponentEndOverlap`
  (params (OverlappedComponent :type "PrimitiveComponent Object Reference") (OtherActor :type "Actor Object Reference") (OtherComp :type "PrimitiveComponent Object Reference") (OtherBodyIndex :type Integer))
  ; Close The Door If The Player Exit The Box
  (cast `/Game/ThirdPerson/Blueprints/BP_ThirdPersonCharacter` OtherActor)
  (`TimelineComponent.Reverse` (`self.TL_Door`)))

(fn `UserConstructionScript`)