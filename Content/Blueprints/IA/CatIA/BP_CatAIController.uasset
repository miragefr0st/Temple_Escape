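; AI controller for the cat that turns perception events into a blackboard target and drives the cat's detection widget.
; Player noises fill a detection gauge through a curve fed by DistanceHearingMultiplier, updating the progress bar and targeting the player when full.
; Other senses switch the target unless SensedActorIsPlayer holds, or clear it when sensing fails, resetting the gauge in both cases without refreshing the bar.
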(event `self.ReceiveBeginPlay`
  (`KismetSystemLibrary.Delay` 0.2)
  (bind _asbp_cat (cast `/Game/Blueprints/IA/CatIA/BP_Cat` (`self.K2_GetPawn`)))
  (bind _aswbp_cat_detection (cast `/Game/Blueprints/IA/CatIA/WBP_CatDetection` (`WidgetComponent.GetUserWidgetObject` (`/Game/Blueprints/IA/CatIA/BP_Cat.Widget` _asbp_cat))))
  (set `self.DetectionWidget` _aswbp_cat_detection)
  (`KismetSystemLibrary.PrintString` "got widget"))

(event `self.AIPerception.OnTargetPerceptionUpdated`
  (params (Actor :type "Actor Object Reference") (Stimulus :type "AIStimulus Structure"))
  (bind (_age _expirationage _strength _stimuluslocation _receiverlocation _tag _bsuccessfullysensed) (break `AIStimulus` Stimulus))
  (bind _progressbar_19 (`/Game/Blueprints/IA/CatIA/WBP_CatDetection.ProgressBar_19` (`self.DetectionWidget`)))
  (bind _returnvalue (`AIPerceptionSystem.GetSenseClassForStimulus` Stimulus))
  (if (== _returnvalue "/Script/AIModule.AISense_Hearing")
    ; Increament DetectionGauge(0->100)
    (if (== (`GameplayStatics.GetPlayerCharacter` 0) Actor)
      (bind _output_get (set `self.DetectionGauge` (+ (`self.DetectionGauge`) (* (`CurveFloat.GetFloatValue` (`self.Curve`) (`self.DistanceHearingMultiplier` _strength _stimuluslocation)) 20.0))))
      (`/Engine/EditorBlueprintResources/StandardMacros.IsValid` _progressbar_19
        (:`Is Valid`
          (set `ProgressBar.Percent` (/ _output_get 100.0) _progressbar_19))
        (:`Is Not Valid`
          _))
      (if (>= (`self.DetectionGauge`) 100.0)
        (`BlackboardComponent.SetValueAsObject` (`AIBlueprintHelperLibrary.GetBlackboard` null) (`|GetArrayItem` (`self.BBKeyNames`)) (`GameplayStatics.GetPlayerCharacter` 0))))
    (elif _bsuccessfullysensed
      (if (`self.SensedActorIsPlayer`)
        (`KismetSystemLibrary.PrintString` "Focused on player")
        (else
          (`BlackboardComponent.SetValueAsObject` (`AIBlueprintHelperLibrary.GetBlackboard` null) (`|GetArrayItem` (`self.BBKeyNames`)) Actor)
          (`KismetSystemLibrary.PrintString` "Switched Target")
          (set `self.DetectionGauge` 0.0)))
      (else
        (`BlackboardComponent.SetValueAsObject` (`AIBlueprintHelperLibrary.GetBlackboard` null) (`|GetArrayItem` (`self.BBKeyNames`)) (`self.EmptyActor`))
        (`KismetSystemLibrary.PrintString` "forgot")
        (set `self.DetectionGauge` 0.0)))))

(event `self.AIPerception.OnTargetPerceptionForgotten`
  (params (Actor :type "Actor Object Reference")))

(fn `UserConstructionScript`)