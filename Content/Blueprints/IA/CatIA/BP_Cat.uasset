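; BP_Cat is an AI-controlled cat character that patrols using a behavior tree.
; On BeginPlay its AI controller runs BT_Cat, then the Blueprint writes the first Patrol point location to the blackboard key named by the first KeyNames entry.
; The Blueprint holds no other active logic, so any further behavior is left to the tree.
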(event `self.ReceiveBeginPlay`
  (`AIController.RunBehaviorTree` (`AIBlueprintHelperLibrary.GetAIController` self) "/Game/Blueprints/IA/CatIA/BT_Cat.BT_Cat")
  (`BlackboardComponent.SetValueAsVector` (`AIBlueprintHelperLibrary.GetBlackboard` null) (`|GetArrayItem` (`self.KeyNames`)) (`|GetArrayItem` (`/Game/Blueprints/IA/CatIA/BP_PatrolRoute.PatrolPointsLocations` (`self.Patrol`)))))

(fn `UserConstructionScript`)