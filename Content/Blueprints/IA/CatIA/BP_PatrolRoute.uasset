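; Patrol route actor, filed under cat AI, that turns placed patrol point actors into a stored list of world locations.
; The construction script attaches each point actor to the route, keeping its world transform.
; On BeginPlay it caches valid points' locations at matching indices, has each bind to its destroy event, fires that event and clears the actor array.
; Only the locations remain at runtime, with the point actors serving as placement markers.
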(event `self.ReceiveBeginPlay`
  (for (_array_element _array_index) (`self.PatrolPointsActors`)
    (`/Engine/EditorBlueprintResources/StandardMacros.IsValid` _array_element
      (:`Is Valid`
        (`KismetArrayLibrary.Array_Set` (`self.PatrolPointsLocations`) _array_index (`self.K2_GetActorLocation` _array_element) true)
        (`/Game/Blueprints/IA/CatIA/BP_PatrolPoints.BindDestroyEvent` _array_element self))))
  (`self.EventDestroyPoints`)
  (`KismetArrayLibrary.Array_Clear` (`self.PatrolPointsActors`)))

(fn `UserConstructionScript`
  (for _array_element (`self.PatrolPointsActors`)
    (`self.K2_AttachToActor` _array_element self "None" "KeepWorld" "KeepWorld" "KeepWorld" false)))