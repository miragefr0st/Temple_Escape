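; BP_FlyingZone is a zone actor that supplies random points inside its collision component's bounds, apparently for flying AI.
; GetRandomPoint picks random X, Y and Z values within the component's box extent, centered on the actor location.
; GetPointInNavMesh repeatedly draws such points until one projects onto the navigation mesh, then returns the projected location, with no retry limit.
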(event `self.ReceiveBeginPlay`
  (set `self.Box Extent` (`.BoxExtent` (`KismetSystemLibrary.GetComponentBounds` (`self.CollisionComponent`))))
  (set `self.ActorLocation` (`self.K2_GetActorLocation`)))

(fn `GetPointInNavMesh`
  (returns (RandomPoint :type "Vector Structure"))
  (set `self.Box Extent` (`.BoxExtent` (`KismetSystemLibrary.GetComponentBounds` (`self.CollisionComponent`))))
  (set `self.ActorLocation` (`self.K2_GetActorLocation`))
  (bind _randompoint (`self.GetRandomPoint` :!label _label))
  (bind (_projectedlocation _returnvalue) (`NavigationSystemV1.K2_ProjectPointToNavigation` _randompoint))
  (if _returnvalue
    (return _projectedlocation)
    (else
      (goto _label))))

(fn `GetRandomPoint`
  (returns (RandomPoint :type "Vector Structure"))
  (bind (_actorlocation_x _actorlocation_y _actorlocation_z) (`KismetMathLibrary.BreakVector` (`self.ActorLocation`)))
  (bind (_box_extent_x _box_extent_y _box_extent_z) (`KismetMathLibrary.BreakVector` (`self.Box Extent`)))
  (bind _actorlocation_x_2 (`KismetMathLibrary.BreakVector` (`self.ActorLocation`)))
  (bind _box_extent_x_2 (`KismetMathLibrary.BreakVector` (`self.Box Extent`)))
  (bind (_actorlocation_x_3 _actorlocation_y_2) (`KismetMathLibrary.BreakVector` (`self.ActorLocation`)))
  (bind (_box_extent_x_3 _box_extent_y_2) (`KismetMathLibrary.BreakVector` (`self.Box Extent`)))
  (set `self.Box Extent` (`.BoxExtent` (`KismetSystemLibrary.GetComponentBounds` (`self.CollisionComponent`))))
  (set `self.ActorLocation` (`self.K2_GetActorLocation`))
  (return (`KismetMathLibrary.MakeVector` (`KismetMathLibrary.RandomFloatInRange` (- _actorlocation_x_2 _box_extent_x_2) (+ _actorlocation_x_2 _box_extent_x_2)) (`KismetMathLibrary.RandomFloatInRange` (- _actorlocation_y_2 _box_extent_y_2) (+ _actorlocation_y_2 _box_extent_y_2)) (`KismetMathLibrary.RandomFloatInRange` (- _actorlocation_z _box_extent_z) (+ _actorlocation_z _box_extent_z)))))

(fn `UserConstructionScript`)