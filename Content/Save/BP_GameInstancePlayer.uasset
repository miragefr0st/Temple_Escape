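; BP_GameInstancePlayer is a Game Instance that keeps player settings and the next scene name or reference available across level changes.
; On Init it sets SM_Master as the base sound mix.
; Getter and setter functions expose the volume, resolution, quality and screen settings as one group, and a separate pair stores and returns NextScene.
; It only holds these values in variables, without applying them or writing them to disk.
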(event `self.ReceiveInit`
  (`GameplayStatics.SetBaseSoundMix` "/Game/SFX/SM_Master.SM_Master"))

(fn `GetNextScene`
  (returns (NextScene :type String))
  (return (`self.NextScene`)))

(fn `GetSettingsPlayer`
  (returns (Volume :type "Float (double-precision)") (Res :type String) (Quality :type Integer) (Screen :type String))
  (return (`self.Volume`) (`self.Res`) (`self.Quality`) (`self.Screen`)))

(fn `SetNewScene`
  (params (NextScene :type String))
  (set `self.NextScene` NextScene))

(fn `SetSettingsPlayer`
  (params (Volume :type "Float (double-precision)") (Res :type String) (Quality :type Integer) (Screen :type String))
  (set `self.Volume` Volume)
  (set `self.Res` Res)
  (set `self.Quality` Quality)
  (set `self.Screen` Screen))