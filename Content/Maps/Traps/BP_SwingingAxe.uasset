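; BP_SwingingAxe is a trap that swings an axe back and forth continuously and kills the player on contact.
; From BeginPlay, a timeline drives the Cylinder's relative yaw through a half turn, reversing or replaying each time it finishes to loop endlessly.
; LeftBlade's begin overlap calls DeathMessage on the overlapping actor if it is the player character; no other blade has overlap logic here.
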(event `self.ReceiveBeginPlay`
  (`self.AxeSwing`))

(event `AxeSwing`
  (set `self.Direction` "Forward")
  (bind (_direction _newtrack_0) (`Timeline|AxeSwingTimeline` :!label _label)
    (:`Update`
      (`SceneComponent.K2_SetRelativeRotation` (`self.Cylinder`) (`KismetMathLibrary.MakeRotator` 0.0 0.0 (`KismetMathLibrary.Lerp` 0.0 180.0 _newtrack_0)) false false))
    (:`Finished`
      (if (`|EnumEquality` _direction "Forward")
        (`self.ReverseAxeSwing`)
        (else
          (`self.AxeSwing`))))))

(event `ReverseAxeSwing`
  (set `self.Direction` "Backward")
  (goto _label :!via `Reverse`))

(event `self.LeftBlade.OnComponentBeginOverlap`
  (params (OverlappedComponent :type "PrimitiveComponent Object Reference") (OtherActor :type "Actor Object Reference") (OtherComp :type "PrimitiveComponent Object Reference") (OtherBodyIndex :type Integer) (bFromSweep :type Boolean) (SweepResult :type "HitResult Structure (by ref)"))
  (if (== OtherActor (`GameplayStatics.GetPlayerCharacter` 0))
    (message `/Game/ThirdPerson/Blueprints/BPI_CharacterInterface.Death` OtherActor)))

(fn `UserConstructionScript`)