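; BP_ObjectToFollow is an actor in the BlazingGear map that travels along the spline of a referenced PatrolRoute.
; On BeginPlay it starts a timeline with its play rate set to one over TimeTComplete, so that variable controls the traversal time.
; Each update maps the timeline's MoveTrack to a distance along the spline and sets the actor's world location and rotation from that point.
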(event `self.ReceiveBeginPlay`
  (`self.Move Object`))

(event `Move Object`
  (bind _patrolroute (`/Game/Maps/BlazingGear/BP_PatrolRoute.PatrolRoute` (`self.PatrolRoute`)))
  (`TimelineComponent.SetPlayRate` (`self.TimelineVar`) (/ 1.0 (`self.timeTComplete`)))
  (bind (_direction _move_track) (`Timeline|TimelineVar`)
    (:`Update`
      (bind _returnvalue (`KismetMathLibrary.Lerp` 0.0 (`SplineComponent.GetSplineLength` _patrolroute) _move_track))
      (`self.K2_SetActorLocationAndRotation` (`SplineComponent.GetLocationAtDistanceAlongSpline` _patrolroute _returnvalue "World") (`SplineComponent.GetRotationAtDistanceAlongSpline` _patrolroute _returnvalue "World")))))

(fn `UserConstructionScript`)