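; BP_Explication is a trigger object that pauses the game to show an explanation panel when the player walks into it.
; When BP_ThirdPersonCharacter overlaps Area and NbPassage is zero, a short delay precedes creating W_ExplicationPannels and enabling the cursor and UI input.
; CloseWidget removes the panel and restores game-only input and play.
; The step setting NbPassage is unconnected, so this graph never blocks repeat displays.
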(event `self.Area.OnComponentBeginOverlap`
  (params (OverlappedComponent :type "PrimitiveComponent Object Reference") (OtherActor :type "Actor Object Reference") (OtherComp :type "PrimitiveComponent Object Reference") (OtherBodyIndex :type Integer) (bFromSweep :type Boolean) (SweepResult :type "HitResult Structure (by ref)"))
  (bind _returnvalue (`GameplayStatics.GetPlayerController` 0))
  (if (== (`self.nbPassage`) 0)
    (cast `/Game/ThirdPerson/Blueprints/BP_ThirdPersonCharacter` OtherActor)
    (`KismetSystemLibrary.Delay` 0.4)
    (bind _returnvalue_2 (`|CreateWidget` "/Game/Maps/BlazingGear/UI/W_ExplicationPannels.W_ExplicationPannels_C" (`GameplayStatics.GetPlayerController` 0)))
    (bind _output_get (set `self.ExplainWidget` _returnvalue_2))
    (`UserWidget.AddToViewport` _output_get 0)
    (`WidgetBlueprintLibrary.SetInputMode_GameAndUIEx` _returnvalue _output_get)
    (set `PlayerController.bShowMouseCursor` true _returnvalue)
    (`GameplayStatics.SetGamePaused` true)))

(event `self.Area.OnComponentEndOverlap`
  (params (OverlappedComponent :type "PrimitiveComponent Object Reference") (OtherActor :type "Actor Object Reference") (OtherComp :type "PrimitiveComponent Object Reference") (OtherBodyIndex :type Integer)))

(fn `CloseWidget`
  (bind _returnvalue (`GameplayStatics.GetPlayerController` 0))
  (`Widget.RemoveFromParent` (`self.ExplainWidget`))
  (`WidgetBlueprintLibrary.SetInputMode_GameOnly` _returnvalue)
  (set `PlayerController.bShowMouseCursor` false _returnvalue)
  (`GameplayStatics.SetGamePaused` false))

(fn `UserConstructionScript`)