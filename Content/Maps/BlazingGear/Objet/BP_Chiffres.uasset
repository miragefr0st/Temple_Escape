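; BP_Chiffres is the Roman numeral display for a code dial puzzle in the BlazingGear map.
; On BeginPlay it binds to the turn-left, turn-right and reset events of the first BP_Cadran found.
; Turns step a counter clamped to 1–9 and update the numeral text, while reset clears only the selected code and entered-code text.
; Two helper functions report whether the displayed numeral is at either limit.
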(event `self.ReceiveBeginPlay`
  (bind _returnvalue (`GameplayStatics.GetActorOfClass` "/Game/Maps/BlazingGear/Objet/BP_Cadran.BP_Cadran_C"))
  (add `/Game/Maps/BlazingGear/Objet/BP_Cadran.ActivateChangeNumberLeft` _returnvalue (delegate `TurnLeftEvent`))
  (add `/Game/Maps/BlazingGear/Objet/BP_Cadran.ActivateChangeNumberRight` _returnvalue (delegate `TurnRightEvent`))
  (add `/Game/Maps/BlazingGear/Objet/BP_Cadran.ResetCode` _returnvalue (delegate `ResetCodeEvent`)))

(event `TurnRightEvent`
  (`self.changeNumber` 1))

(event `ResetCodeEvent`
  (bind _codesaisie (`self.CodeSaisie`))
  (set `self.CodeSelected` "")
  (`TextRenderComponent.K2_SetText` _codesaisie (`KismetTextLibrary.Conv_StringToText` ""))
  (`KismetSystemLibrary.PrintString` (`KismetTextLibrary.Conv_TextToString` (`TextRenderComponent.Text` _codesaisie))))

(event `TurnLeftEvent`
  (`self.changeNumber` -1))

(event `self.ReceiveTick`
  (params (DeltaSeconds :type "Float (single-precision)")))

(fn `changeNumber`
  (params (index :type Integer))
  (locals (romanNumber :type Integer :default 7))
  (bind _returnvalue (+ (`self.compteur`) index))
  ;[0.15 0.15 0.15 0.5 13] si index = 1 ou -1
  (if (or (== index -1) (== index 1))
    ;[0.15 0.15 0.15 0.5 13] Alors affectation de l'index au romanNumber, sans que celui ci soit en dehors de [1;9]
    (if (and (> _returnvalue 0) (< _returnvalue 10))
      (bind _output_get (set `self.compteur` _returnvalue))
      (`self.NumberToRomanNumber` _output_get)
      (else
        (`KismetSystemLibrary.PrintString` "Hello")))))

(fn `hasReacchedMaxLimit`
  (returns (limitReached :type Boolean))
  (return (`KismetTextLibrary.EqualEqual_TextText` (`TextRenderComponent.Text` (`self.Numbers`)) "IX")))

(fn `hasReacchedMinLimit`
  (returns (limitReached :type Boolean))
  (return (`KismetTextLibrary.EqualEqual_TextText` (`TextRenderComponent.Text` (`self.Numbers`)) "I")))

(fn `NumberToRomanNumber`
  (params (Number :type Integer))
  (if (== Number 1)
    (`TextRenderComponent.K2_SetText` (`self.Numbers`) (`KismetTextLibrary.Conv_StringToText` "I"))
    (elif (== Number 2)
      (`TextRenderComponent.K2_SetText` (`self.Numbers`) (`KismetTextLibrary.Conv_StringToText` "II"))
      (elif (== Number 3)
        (`TextRenderComponent.K2_SetText` (`self.Numbers`) (`KismetTextLibrary.Conv_StringToText` "III"))
        (elif (== Number 4)
          (`TextRenderComponent.K2_SetText` (`self.Numbers`) (`KismetTextLibrary.Conv_StringToText` "IV"))
          (elif (== Number 5)
            (`TextRenderComponent.K2_SetText` (`self.Numbers`) (`KismetTextLibrary.Conv_StringToText` "V"))
            (elif (== Number 6)
              (`TextRenderComponent.K2_SetText` (`self.Numbers`) (`KismetTextLibrary.Conv_StringToText` "VI"))
              (elif (== Number 7)
                (`TextRenderComponent.K2_SetText` (`self.Numbers`) (`KismetTextLibrary.Conv_StringToText` "VII"))
                (elif (== Number 8)
                  (`TextRenderComponent.K2_SetText` (`self.Numbers`) (`KismetTextLibrary.Conv_StringToText` "VIII"))
                  (elif (== Number 9)
                    (`TextRenderComponent.K2_SetText` (`self.Numbers`) (`KismetTextLibrary.Conv_StringToText` "IX"))))))))))))

(fn `UserConstructionScript`)