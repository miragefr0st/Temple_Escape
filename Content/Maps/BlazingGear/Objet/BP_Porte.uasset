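; Code-locked door for the BlazingGear map that reacts to codes sent by the BP_Chiffres actor.
; On BeginPlay it finds that actor by class and binds to its SendCodeToDoor dispatcher.
; A code matching CodeToFind hides the Plane component, changing visibility only.
; A wrong code prints a colored debug message revealing the expected and entered codes.
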(event `self.ReceiveBeginPlay`
  (bind _returnvalue (`GameplayStatics.GetActorOfClass` "/Game/Maps/BlazingGear/Objet/BP_Chiffres.BP_Chiffres_C"))
  (add `/Game/Maps/BlazingGear/Objet/BP_Chiffres.SendCodeToDoor` _returnvalue (delegate `CustomEvent`))
  (`KismetSystemLibrary.PrintString` "Binding Door"))

(event `CustomEvent`
  (params (CodeToSend :type String))
  (bind _codetofind (`self.CodeToFind`))
  (if (`KismetStringLibrary.EqualEqual_StrStr` CodeToSend _codetofind)
    (`SceneComponent.SetVisibility` (`self.Plane`) false false)
    (`KismetSystemLibrary.PrintString` "Code ok ")
    (else
      (`KismetSystemLibrary.PrintString` (`KismetStringLibrary.Concat_StrStr` "Le bon code etait " _codetofind "-- Saisie : " CodeToSend) true true (struct :`R` 1.0 :`B` 0.241287 :`A` 1.0) 3.0))))

(fn `UserConstructionScript`)