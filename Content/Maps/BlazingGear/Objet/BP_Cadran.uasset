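; Dial actor for the BlazingGear map that turns its Roue2 wheel left or right, apparently as part of a number puzzle.
; After a short delay, BeginPlay turns it right once, then binds handlers to the turn dispatchers.
; Turns increment NbEssaie and fire number-change dispatchers; TurnLeft/TurnRight use fixed steps, while bound handlers add current world yaw plus an offset as the delta.
; A separate Rotate function makes finer turns without counting.
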(event `self.ReceiveBeginPlay`
  (`KismetSystemLibrary.Delay` 1.0)
  (`self.TurnRight`)
  (add `self.TurnRightEvent` (delegate `TImelineTurnRight`))
  (add `self.TurnLeftEvent` (delegate `TimelineTurnLeft`)))

(event `TImelineTurnRight`
  (bind (_returnvalue_roll _returnvalue_pitch _returnvalue_yaw) (`KismetMathLibrary.BreakRotator` (`SceneComponent.K2_GetComponentRotation` (`self.Roue2`))))
  (`SceneComponent.K2_AddLocalRotation` (`self.Roue2`) (`KismetMathLibrary.MakeRotator` 0.0 0.0 (+ _returnvalue_yaw 30.0)) false false)
  (set `self.nbEssaie` (+ (`self.nbEssaie`) 1))
  (`self.ActivateChangeNumberRight`))

(event `TimelineTurnLeft`
  (bind (_returnvalue_roll _returnvalue_pitch _returnvalue_yaw) (`KismetMathLibrary.BreakRotator` (`SceneComponent.K2_GetComponentRotation` (`self.Roue2`))))
  (`SceneComponent.K2_AddLocalRotation` (`self.Roue2`) (`KismetMathLibrary.MakeRotator` 0.0 0.0 (+ _returnvalue_yaw -30.0)) false false)
  (set `self.nbEssaie` (+ (`self.nbEssaie`) 1))
  (`self.ActivateChangeNumberLeft`))

(event `self.ReceiveTick`
  (params (DeltaSeconds :type "Float (single-precision)")))

(event `BindToRightTurn_E`)

(event `BindToLeftTurn_E`)

(fn `rotate`
  (params (Left_Right :type Integer))
  (bind _returnvalue (`GameplayStatics.GetActorOfClass` "/Game/Maps/BlazingGear/Objet/BP_Chiffres.BP_Chiffres_C"))
  (if (== Left_Right -1)
    (`SceneComponent.K2_AddLocalRotation` (`self.Roue2`) (struct :`Yaw` -5.0) false false)
    (elif (== Left_Right 1)
      (`SceneComponent.K2_AddLocalRotation` (`self.Roue2`) (struct :`Yaw` 5.0) false false))))

(fn `TurnLeft`
  (`SceneComponent.K2_AddLocalRotation` (`self.Roue2`) (struct :`Yaw` -30.0) false false)
  (set `self.nbEssaie` (+ (`self.nbEssaie`) 1))
  (`self.ActivateChangeNumberLeft`))

(fn `TurnRight`
  (`SceneComponent.K2_AddLocalRotation` (`self.Roue2`) (struct :`Yaw` 30.0) false false)
  (set `self.nbEssaie` (+ (`self.nbEssaie`) 1))
  (`self.ActivateChangeNumberRight`))

(fn `UserConstructionScript`)