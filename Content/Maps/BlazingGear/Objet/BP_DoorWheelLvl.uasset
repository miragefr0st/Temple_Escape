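; A trigger-box door for the BlazingGear map that opens when the third-person character enters and closes when they leave.
; On entry, four Niagara effects activate in a delayed sequence before the door timeline plays; leaving reverses the timeline.
; The timeline update lerps the Cylinder's relative yaw and location toward OpenAngle and OpenPos.
; All door effects are deactivated at BeginPlay, and ActivateNiagaras is an empty stub.
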(event `self.ReceiveBeginPlay`
  (`ActorComponent.Deactivate` (`self.NiagaraDoor`))
  (`ActorComponent.Deactivate` (`self.N_DustDoorNiagara`))
  (`ActorComponent.Deactivate` (`self.NiagaraDoor2`))
  (`ActorComponent.Deactivate` (`self.NiagaraDoor1`))
  (`ActorComponent.Deactivate` (`self.NiagaraDoor3`)))

(event `self.Box.OnComponentBeginOverlap`
  (params (OverlappedComponent :type "PrimitiveComponent Object Reference") (OtherActor :type "Actor Object Reference") (OtherComp :type "PrimitiveComponent Object Reference") (OtherBodyIndex :type Integer) (bFromSweep :type Boolean) (SweepResult :type "HitResult Structure (by ref)"))
  ; Open The Door if The Player Overlap the Box
  (cast `/Game/ThirdPerson/Blueprints/BP_ThirdPersonCharacter` OtherActor)
  (`KismetSystemLibrary.Delay` 0.3)
  (`ActorComponent.Activate` (`self.NiagaraDoor`) false)
  (`KismetSystemLibrary.Delay` 0.3)
  (`ActorComponent.Activate` (`self.NiagaraDoor1`) false)
  (`KismetSystemLibrary.Delay` 0.3)
  (`ActorComponent.Activate` (`self.NiagaraDoor2`) false)
  (`KismetSystemLibrary.Delay` 0.3)
  (`ActorComponent.Activate` (`self.NiagaraDoor3`) false)
  (`KismetSystemLibrary.Delay` 0.2)
  (`TimelineComponent.Play` (`self.TL_Door`)))

(event `self.Box.OnComponentEndOverlap`
  (params (OverlappedComponent :type "PrimitiveComponent Object Reference") (OtherActor :type "Actor Object Reference") (OtherComp :type "PrimitiveComponent Object Reference") (OtherBodyIndex :type Integer))
  ; Close The Door If The Player Exit The Box
  (cast `/Game/ThirdPerson/Blueprints/BP_ThirdPersonCharacter` OtherActor)
  (`TimelineComponent.Reverse` (`self.TL_Door`)))

(fn `ActivateNiagaras`)

(fn `UserConstructionScript`)