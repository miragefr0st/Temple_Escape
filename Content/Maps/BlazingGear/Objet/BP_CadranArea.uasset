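; BP_CadranArea is a trigger box that opens the dial UI (WCadranUI) for code entry in the BlazingGear map.
; Overlap start clears the BP_Chiffres number and entered-code texts, adds the widget to the viewport and focuses it in Game and UI input mode with the cursor shown.
; Overlap end removes the widget, resets the entered code and hides the cursor, but leaves the input mode unchanged.
; Neither event filters the overlapping actor.
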(event `self.Box.OnComponentBeginOverlap`
  (params (OverlappedComponent :type "PrimitiveComponent Object Reference") (OtherActor :type "Actor Object Reference") (OtherComp :type "PrimitiveComponent Object Reference") (OtherBodyIndex :type Integer) (bFromSweep :type Boolean) (SweepResult :type "HitResult Structure (by ref)"))
  (bind _returnvalue (`GameplayStatics.GetPlayerController` 0))
  (bind _returnvalue_2 (`GameplayStatics.GetActorOfClass` "/Game/Maps/BlazingGear/Objet/BP_Chiffres.BP_Chiffres_C"))
  (`TextRenderComponent.K2_SetText` (`/Game/Maps/BlazingGear/Objet/BP_Chiffres.Numbers` _returnvalue_2) "")
  (`TextRenderComponent.K2_SetText` (`/Game/Maps/BlazingGear/Objet/BP_Chiffres.CodeSaisie` _returnvalue_2) "")
  (bind _returnvalue_3 (`|CreateWidget` "/Game/Maps/BlazingGear/UI/WCadranUI.WCadranUI_C"))
  (set `self.UIChoice` _returnvalue_3)
  (`UserWidget.AddToViewport` _returnvalue_3 0)
  (`WidgetBlueprintLibrary.SetInputMode_GameAndUIEx` _returnvalue _returnvalue_3)
  (set `PlayerController.bShowMouseCursor` true _returnvalue))

(event `self.Box.OnComponentEndOverlap`
  (params (OverlappedComponent :type "PrimitiveComponent Object Reference") (OtherActor :type "Actor Object Reference") (OtherComp :type "PrimitiveComponent Object Reference") (OtherBodyIndex :type Integer))
  (`Widget.RemoveFromParent` (`self.UIChoice`))
  (bind _returnvalue (`GameplayStatics.GetActorOfClass` "/Game/Maps/BlazingGear/Objet/BP_Chiffres.BP_Chiffres_C"))
  (`TextRenderComponent.K2_SetText` (`/Game/Maps/BlazingGear/Objet/BP_Chiffres.CodeSaisie` _returnvalue) (`KismetTextLibrary.Conv_StringToText` ""))
  (set `/Game/Maps/BlazingGear/Objet/BP_Chiffres.CodeSelected` "" _returnvalue)
  (set `PlayerController.bShowMouseCursor` false (`GameplayStatics.GetPlayerController` 0)))

(fn `UserConstructionScript`)