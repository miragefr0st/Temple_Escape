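; Patrol route Blueprint that supplies spline points for an AI to follow back and forth.
; IncrementPatrolRoute steps PatrolIndex by Direction along the PatrolRoute spline and flips Direction at the first and last points, giving a ping-pong path rather than a loop.
; GetSplinePointAsWorldPosition returns the world location of the current point.
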(event `IncrementPatrolRoute`
  ;[0.15 0.15 0.15 0.5 10] Incrémente l'index du prochian point que va suivre l'IA
  ;[0.15 0.15 0.15 0.5 14] Incréméntation de l'index dans la spline
  (bind _output_get (set `self.PatrolIndex` (+ (`self.PatrolIndex`) (`self.Direction`))))
  ;[0.15 0.15 0.15 0.5 14] Vérifie si on est sur le dernier point du spline
  (if (== _output_get (- (`SplineComponent.GetNumberOfSplinePoints` (`self.PatrolRoute`)) 1))
    ;[0.15 0.15 0.15 0.5 14] Direction set à -1 pour faire demi-tour
    (set `self.Direction` -1)
    (else
      ;[0.15 0.15 0.15 0.5 14] Sinon si on est de retour sur le 1er point on avance vers le 2e ect
      (if (== (`self.PatrolIndex`) 0)
        (set `self.Direction` 1)))))

(fn `GetSplinePointAsWorldPosition`
  (returns (Location :type "Vector Structure"))
  ;[0.15 0.15 0.15 0.5 12] Connaitre la position d'un point du spline, dans le monde
  (return (`SplineComponent.GetLocationAtSplinePoint` (`self.PatrolRoute`) (`self.PatrolIndex`) "World")))

(fn `UserConstructionScript`)