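; BP_LandMine is a land mine actor that kills a player character on overlap.
; The Explosion component is deactivated on BeginPlay and activated when a BP_ThirdPersonCharacter overlaps the mine.
; After a short delay it calls PlayerDeath on the stored character, then destroys itself after a second delay.
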(event `self.ReceiveBeginPlay`
  (`ActorComponent.Deactivate` (`self.Explosion`)))

(event `self.ReceiveActorBeginOverlap`
  (params (OtherActor :type "Actor Object Reference"))
  (bind _asbp_third_person_character (cast `/Game/ThirdPerson/Blueprints/BP_ThirdPersonCharacter` OtherActor))
  (set `self.As BP Third Person Character` _asbp_third_person_character)
  (`ActorComponent.Activate` (`self.Explosion`) true)
  (`KismetSystemLibrary.Delay` 0.2)
  (`/Game/ThirdPerson/Blueprints/BP_ThirdPersonCharacter.PlayerDeath` (`self.As BP Third Person Character`))
  (`KismetSystemLibrary.Delay` 0.2)
  (`self.K2_DestroyActor`))

(fn `UserConstructionScript`)